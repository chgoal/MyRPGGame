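; AI controller for the boss that turns perception updates into blackboard state.
; BeginPlay resets BaseAction and casts its owner to BP_Boss; sighting a Player-tagged actor sets FindEnemy, EnemyActor and a new BaseAction.
; Losing sight clears the enemy keys and requests a movement prediction, but the PredictSense handler storing that location is disconnected.
; ConfirmEnemy sets EnemyActor directly, while SightSense is an uncalled variant using ActionEnemyActor.
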(event OnTargetPerceptionUpdated(PerceptionComponent)
  (params (Actor :type Actor%20Object%20Reference) (Stimulus :type AI%20Stimulus%20Structure))
  (bind _returnvalue (AI|GetBlackboard 0))
  (bind _returnvalue_2 (Utilities|Name|MakeLiteralName "EnemyActor"))
  (bind _returnvalue_3 (AI|GetBlackboard 0))
  (bind _returnvalue_4 (Utilities|Name|MakeLiteralName "FindEnemy"))
  (Utilities|FlowControl|Sequence
    (:then_0
      (bind _returnvalue_5 (Class|AIPerceptionSystem|GetSenseClassforStimulus Stimulus))
      (if (and (== _returnvalue_5 "/Script/AIModule.AISense_Sight") (Actor|ActorHasTag Actor "Player"))
        (if (.bSuccessfullySensed (Utilities|Struct|BreakAIStimulus Stimulus))
          (AI|Components|Blackboard|SetValueasBool _returnvalue_3 _returnvalue_4 true)
          (AI|Components|Blackboard|SetValueasObject _returnvalue _returnvalue_2 Actor)
          (AI|Components|Blackboard|SetValueasEnum (AI|GetBlackboard 0) (Utilities|Name|MakeLiteralName "BaseAction") 1)
          (else
            (AI|Components|Blackboard|SetValueasBool _returnvalue_3 _returnvalue_4 false)
            (AI|Components|Blackboard|SetValueasObject _returnvalue _returnvalue_2 0)
            (Class|AISensePrediction|RequestPawnPredictionEvent (Pawn|GetControlledPawn) Actor 0.5)))))))

(event EventBeginPlay
  (AI|Components|Blackboard|SetValueasEnum (AI|GetBlackboard 0) (Utilities|Name|MakeLiteralName "BaseAction"))
  (bind _asbp_boss (Utilities|Casting|CastToBP_Boss (Components|GetOwner)))
  (Variables|Default|SetBoss _asbp_boss))

(event EventTick
  (params (DeltaSeconds :type Float%20%28single-precision%29)))

(fn ConstructionScript)

(fn SightSense
  (params (Actor :type Actor%20Object%20Reference) (Stimulus :type AI%20Stimulus%20Structure))
  (bind _returnvalue (AI|GetBlackboard 0))
  (bind _returnvalue_2 (Utilities|Name|MakeLiteralName "ActionEnemyActor"))
  (bind _returnvalue_3 (AI|GetBlackboard 0))
  (bind _returnvalue_4 (Utilities|Name|MakeLiteralName "FindEnemy"))
  (bind _returnvalue_5 (Class|AIPerceptionSystem|GetSenseClassforStimulus Stimulus))
  (if (and (== _returnvalue_5 "/Script/AIModule.AISense_Sight") (Actor|ActorHasTag Actor "Player"))
    (if (.bSuccessfullySensed (Utilities|Struct|BreakAIStimulus Stimulus))
      ;[1 1 1] 之后直接修改为玩家
      (AI|Components|Blackboard|SetValueasBool _returnvalue_3 _returnvalue_4 true)
      (AI|Components|Blackboard|SetValueasObject _returnvalue _returnvalue_2 Actor)
      (AI|Components|Blackboard|SetValueasEnum (AI|GetBlackboard 0) (Utilities|Name|MakeLiteralName "BaseAction") 1)
      (else
        (AI|Components|Blackboard|SetValueasBool _returnvalue_3 _returnvalue_4 false)
        (AI|Components|Blackboard|SetValueasObject _returnvalue _returnvalue_2 0)
        (Class|AISensePrediction|RequestPawnPredictionEvent (Pawn|GetControlledPawn) Actor 0.5)))
    (return)))

(fn PredictSense
  (params (Actor :type Actor%20Object%20Reference) (Stimulus :type AI%20Stimulus%20Structure%20%28by%20ref%29))
  (bind (_age _expirationage _strength _stimuluslocation _receiverlocation _tag _bsuccessfullysensed) (Utilities|Struct|BreakAIStimulus Stimulus))
  (bind _returnvalue (Class|AIPerceptionSystem|GetSenseClassforStimulus Stimulus))
  (if (== _returnvalue "/Script/AIModule.AISense_Prediction")
    (if (and (Actor|ActorHasTag Actor "Player") _bsuccessfullysensed)
      (AI|Components|Blackboard|SetValueasVector (AI|GetBlackboard 0) (Utilities|Name|MakeLiteralName "LastActVector") _stimuluslocation))
    (return)))

(fn ConfirmEnemy
  (params (Actor :type Actor%20Object%20Reference))
  (AI|Components|Blackboard|SetValueasObject (AI|GetBlackboard 0) (Utilities|Name|MakeLiteralName "EnemyActor") Actor)
  (return))