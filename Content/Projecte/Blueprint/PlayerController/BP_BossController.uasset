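; Boss controller that turns AI perception updates into blackboard values.
; BeginPlay resets the patrol-style PointIndex; each perception update sets FindEnemy true only for a successful sight of a Player-tagged actor, otherwise false, including on noise events.
; Sensed "Noise" stimuli store their location in NoisePosition, while other sensed stimuli from a BP_Player store that actor as Enemy.
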(event OnTargetPerceptionUpdated(PerceptionComponent)
  (params (Actor :type Actor%20Object%20Reference) (Stimulus :type AI%20Stimulus%20Structure))
  (bind (_age _expirationage _strength _stimuluslocation _receiverlocation _tag _bsuccessfullysensed) (Utilities|Struct|BreakAIStimulus Stimulus))
  (CallFunction|SightSense Actor Stimulus)
  (if (Utilities|Name|Equal(Name) _tag "Noise")
    (if _bsuccessfullysensed
      (AI|Components|Blackboard|SetValueasVector (AI|GetBlackboard 0) (Variables|Default|GetNoisePosition) _stimuluslocation))
    (elif _bsuccessfullysensed
      (Utilities|Casting|CastToBP_Player Actor)
      (AI|Components|Blackboard|SetValueasObject (AI|GetBlackboard 0) (Variables|Default|GetEnemy) Actor))))

(event EventBeginPlay
  (Class|BlackboardComponent|SetValueasInt (AI|GetBlackboard 0) (Utilities|Name|MakeLiteralName "PointIndex")))

(event EventTick
  (params (DeltaSeconds :type Float%20%28single-precision%29)))

(fn ConstructionScript)

(fn SightSense
  (params (Actor :type Actor%20Object%20Reference) (Stimulus :type AI%20Stimulus%20Structure))
  (bind _returnvalue (AI|GetBlackboard 0))
  (bind _returnvalue_2 (Utilities|Name|MakeLiteralName "FindEnemy"))
  (bind _returnvalue_3 (Class|AIPerceptionSystem|GetSenseClassforStimulus Stimulus))
  (if (Math|Boolean|ANDBoolean (== _returnvalue_3 "/Script/AIModule.AISense_Sight") (Actor|ActorHasTag Actor "Player") (.bSuccessfullySensed (Utilities|Struct|BreakAIStimulus Stimulus)))
    ;[1 1 1] 之后直接修改为玩家
    (AI|Components|Blackboard|SetValueasBool _returnvalue _returnvalue_2 true)
    (else
      (AI|Components|Blackboard|SetValueasBool _returnvalue _returnvalue_2 false))))