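; Player character that drives melee combat, rolling, sprinting and death through the Gameplay Ability System.
; Left attack activates weapon abilities by tag and buffers combo input for SaveAttack; right attack toggles a shield tag.
; The TimeShift macro splits one button into tap-to-roll and hold-to-sprint ("Sprite").
; Tick applies sprint or recharge effects and triggers GA_Death at zero health, while construction slaves modular outfit meshes to the main mesh.
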(event EventBeginPlay)

(event Collision|EventActorBeginOverlap
  (params (OtherActor :type Actor%20Object%20Reference)))

(event EventTick
  (params (DeltaSeconds :type Float%20%28single-precision%29))
  (Utilities|FlowControl|Sequence
    (:then_0
      (CallFunction|Sprite))
    (:then_1
      (CallFunction|LifeorDie))))

(event EventSaveAttack
  (if (Math|Boolean|ANDBoolean (not (Variables|Default|GetbWidgetOpen)) (not (AI|Components|NavMovement|IsFalling (Variables|Character|GetCharacterMovement))) (Utilities|Enum|NotEqual(Enum) (Class|BaseCharacter|GetWeaponState) "EWS_None"))
    (if (Variables|Default|GetbSaveLeftAttack)
      (Variables|Default|SetbSaveLeftAttack false)
      (bind _returnvalue (Class|BaseCharacter|AddedWeaponGameplayTags (Variables|Default|GetWeaponGameplayTag) "LeftAttack"))
      (Abilities|TryActivateAbilitiesbyTag (Variables|Default|GetAbilitySystemComponent) (GameplayTags|MakeGameplayTagContainerfromTag _returnvalue) true))))

(event EventPrintAttribute
  (bind _abilitysystemcomponent (Variables|Default|GetAbilitySystemComponent))
  (bind (_bsuccessfullyfoundattribute _returnvalue) (Ability|Attribute|GetFloatAttributefromAbilitySystemComponent _abilitysystemcomponent "(AttributeName=\"Health\",Attribute=/Script/MyRPGGame.CharacterAttributeSet:Health,AttributeOwner=None)"))
  (if _bsuccessfullyfoundattribute
    (Development|PrintString (Utilities|String|ToString(Float) _returnvalue))))

(event Input|ActionEvents|InputActionLeftAttack
  (params (Key :type Key%20Structure :default "None"))
  (:Pressed
    (if (Math|Boolean|ANDBoolean (not (Variables|Default|GetbWidgetOpen)) (not (AI|Components|NavMovement|IsFalling (Variables|Character|GetCharacterMovement))) (Utilities|Enum|NotEqual(Enum) (Class|BaseCharacter|GetWeaponState) "EWS_None"))
      (if (Variables|Default|GetbLeftAttack)
        (if (Class|PlayerCharacter|GetStartCombo)
          (Variables|Default|SetbSaveLeftAttack true))
        (else
          (Variables|Default|SetbLeftAttack true)
          (bind _returnvalue (Class|BaseCharacter|AddedWeaponGameplayTags (Variables|Default|GetWeaponGameplayTag) "LeftAttack"))
          (Abilities|TryActivateAbilitiesbyTag (Variables|Default|GetAbilitySystemComponent) (GameplayTags|MakeGameplayTagContainerfromTag _returnvalue) true))))))

(event Input|ActionEvents|InputActionRightAttack
  (params (Key :type Key%20Structure :default "None"))
  (bind _tagcontainer (Variables|Default|GetTagContainer))
  (:Pressed
    (Variables|Default|SetbRightAttack true)
    (GameplayTags|AddGameplayTag _tagcontainer "(TagName=\"Ability.Player.Sword.shield\")" :!class /Script/GameplayTags.BlueprintGameplayTagLibrary))
  (:Released
    (Variables|Default|SetbRightAttack false)
    (GameplayTags|RemoveGameplayTag _tagcontainer "(TagName=\"Ability.Player.Sword.shield\")" :!class /Script/GameplayTags.BlueprintGameplayTagLibrary)))

(event Input|ActionEvents|InputActionDoSprite
  (params (Key :type Key%20Structure :default "None"))
  (:Pressed
    (Utilities|TimeShift 0.3 :!label _label
      (:Long
        (Variables|/Script/Engine.CharacterMovementComponent|SetMaxWalkSpeed (Variables|Character|GetCharacterMovement) (Variables|Default|GetSpriteSpeed))
        (GameplayTags|AddGameplayTag (Variables|Default|GetTagContainer) "(TagName=\"Ability.Player.Sword.Sprite\")" :!class /Script/GameplayTags.BlueprintGameplayTagLibrary))
      (:Short
        (if (not (Variables|Default|GetbWidgetOpen))
          (if (not (Variables|Default|GetbSprite))
            (Abilities|TryActivateAbilitybyClass (Variables|Default|GetAbilitySystemComponent) "/Game/Projecte/Blueprint/GAS/GA/GA_Roll.GA_Roll_C" true))))))
  (:Released
    (GameplayTags|RemoveGameplayTag (Variables|Default|GetTagContainer) "(TagName=\"Ability.Player.Sword.Sprite\")" :!class /Script/GameplayTags.BlueprintGameplayTagLibrary)
    (goto _label Released)))

(fn ConstructionScript
  (Class|SkinnedMeshComponent|SetMasterPoseComponent (Variables|Default|GetHead) (Variables|Character|GetMesh) true))

(fn Sprite
  (bind _abilitysystemcomponent (Variables|Default|GetAbilitySystemComponent))
  (bind _returnvalue (Ability|Attribute|GetFloatAttributefromAbilitySystemComponent _abilitysystemcomponent "(AttributeName=\"Stamina\",Attribute=/Script/MyRPGGame.CharacterAttributeSet:Stamina,AttributeOwner=None)"))
  (if (not (Variables|Default|GetbSprite))
    (if (and (> (Math|Vector|VectorLength (Variables|/Script/Engine.MovementComponent|GetVelocity (Variables|Character|GetCharacterMovement))) 0.0) (GameplayTags|HasTag (Variables|Default|GetTagContainer) "(TagName=\"Ability.Player.Sword.Sprite\")" true))
      (if (> _returnvalue 0.0)
        (if (not (AI|Components|NavMovement|IsFalling (Variables|Character|GetCharacterMovement)))
          (GameplayEffects|ApplyGameplayEffectToSelf :self (Variables|Default|GetAbilitySystemComponent) :GameplayEffectClass "/Game/Projecte/Blueprint/GAS/GE/GE_Sprite.GE_Sprite_C" :Level 1.0))
        (else
          (Variables|/Script/Engine.CharacterMovementComponent|SetMaxWalkSpeed (Variables|Character|GetCharacterMovement) (Variables|Default|GetWalkSpeed))
          (GameplayTags|RemoveGameplayTag (Variables|Default|GetTagContainer) "(TagName=\"Ability.Player.Sword.Sprite\")" :!class /Script/GameplayTags.BlueprintGameplayTagLibrary)
          (GameplayEffects|ApplyGameplayEffectToSelf :self (Variables|Default|GetAbilitySystemComponent) :GameplayEffectClass "/Game/Projecte/Blueprint/GAS/GE/GE_Recharge.GE_Recharge_C" :Level 1.0 :!label _label)))
      (elif (< _returnvalue 1e+02)
        (goto _label)))))

(fn ReCharge)

(fn LifeorDie
  (if (<= (.ReturnValue (Ability|Attribute|GetFloatAttributefromAbilitySystemComponent (Variables|Default|GetAbilitySystemComponent) "(AttributeName=\"Health\",Attribute=/Script/MyRPGGame.CharacterAttributeSet:Health,AttributeOwner=None)")) 0.0)
    (if (not (GameplayTags|HasTag (Variables|Default|GetTagContainer) "(TagName=\"Ability.Player.Death\")"))
      (GameplayTags|AddGameplayTag (Variables|Default|GetTagContainer) "(TagName=\"Ability.Player.Death\")" :!class /Script/GameplayTags.BlueprintGameplayTagLibrary)
      (Abilities|TryActivateAbilitybyClass (Variables|Default|GetAbilitySystemComponent) "/Game/Projecte/Blueprint/GAS/GA/GA_Death.GA_Death_C" true))))