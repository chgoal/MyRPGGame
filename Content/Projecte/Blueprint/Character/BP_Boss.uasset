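; BP_Boss is an AI boss character that drives a detection indicator, an overhead health bar and its own death.
; BeginPlay seeds the Blackboard with its spawn location and optional SitActor.
; Tick polls an Ability System attribute, setting a Die tag and Blackboard flag at zero.
; ToDie plays a death montage, then enables ragdoll physics, disables capsule collision and immediately calls DestroyActor on blend-out.
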(event Custom|ToDie
  (bind _mesh (Variables|Character|GetMesh))
  (Animation|Montage|PlayMontage (Variables|Character|GetMesh) "/Game/Projecte/Animation/Enemy/AnimMontage/AM_Death.AM_Death"
    (:OnBlendOut
      (Class|SkeletalMeshComponent|SetAllBodiesSimulatePhysics _mesh true)
      (Class|SkeletalMeshComponent|SetAllBodiesPhysicsBlendWeight _mesh 1.0 false)
      (Collision|SetCollisionEnabled (Variables|Default|GetCapsuleComponent) "NoCollision")
      (Actor|DestroyActor))))

(event Custom|UnFindEnemy
  (params (Value :type Float%20%28single-precision%29))
  (Default|UnRun (CallFunction|GetFindEnemyWiget) Value)
  (if (and (>= Value 0.0) (not (Rendering|IsVisible (Variables|Default|GetFindEnemy))))
    (Rendering|SetVisibility (Variables|Default|GetFindEnemy) true false)
    (elif (<= Value 0.2)
      (Utilities|FlowControl|Delay 0.6)
      (Rendering|SetVisibility (Variables|Default|GetFindEnemy) false false))))

(event Custom|RunFindEnemy
  (params (Value :type Float%20%28single-precision%29))
  (Default|Run (CallFunction|GetFindEnemyWiget) Value)
  (if (and (<= Value 0.9) (not (Rendering|IsVisible (Variables|Default|GetFindEnemy))))
    (Rendering|SetVisibility (Variables|Default|GetFindEnemy) true false)
    (elif (>= Value 0.9)
      (Utilities|FlowControl|Delay 0.6)
      (Rendering|SetVisibility (Variables|Default|GetFindEnemy) false false))))

(event Custom|ResetFindEnemy
  (Rendering|SetVisibility (Variables|Default|GetFindEnemy) false false)
  (Default|ResetMaterial (CallFunction|GetFindEnemyWiget)))

(event EventBeginPlay
  (bind _returnvalue (AI|GetBlackboard 0))
  (bind _sitactor (Variables|Default|GetSitActor))
  (AI|Components|Blackboard|SetValueasVector _returnvalue (Variables|Blackborad|GetActorSpawnLoc) (Transformation|GetActorLocation))
  (Utilities|FlowControl|Sequence
    (:then_0
      (Utilities|IsValid _sitactor
        (:Is%20Valid
          (AI|Components|Blackboard|SetValueasObject _returnvalue (Variables|Blackborad|GetSceneActor) _sitactor))))
    (:then_1
      (Class|BaseCharacter|ReceiveDamage))))

(event Collision|EventActorBeginOverlap
  (params (OtherActor :type Actor%20Object%20Reference)))

(event EventTick
  (params (DeltaSeconds :type Float%20%28single-precision%29))
  (CallFunction|IsDie))

(event EventDamage
  (Default|SetProPercent (CallFunction|GetHeadWigetComponent) (/ (Class|BaseCharacter|GetHealth) (Class|BaseCharacter|GetMaxHeath)))
  (Rendering|SetVisibility (Variables|Default|GetFindEnemy) false false))

(fn ConstructionScript)

(fn IsDie
  (if (<= (.ReturnValue (Ability|Attribute|GetFloatAttributefromAbilitySystemComponent (Variables|Default|GetAbilitySystemComponent) "(AttributeName=\"Health\",Attribute=/Script/MyRPGGame.CharacterAttributeSet:Health,AttributeOwner=None)")) 0.0)
    (if (not (GameplayTags|HasTag (Variables|Default|GetTagContainer) "(TagName=\"Ability.Enemy.Die\")"))
      (GameplayTags|AddGameplayTag (Variables|Default|GetTagContainer) "(TagName=\"Ability.Enemy.Die\")" :!class /Script/GameplayTags.BlueprintGameplayTagLibrary)
      (Variables|Default|SetbIsAlive false)
      (AI|Components|Blackboard|SetValueasBool (AI|GetBlackboard 0) (Variables|Blackborad|GetDie) true))))

(fn GetFindEnemyWiget
  (bind _asui_find_target_widget (Utilities|Casting|CastToUI_FindTargetWidget (UserInterface|GetWidget (Variables|Default|GetFindEnemy))))
  (return _asui_find_target_widget))

(fn GetHeadWigetComponent
  (bind _asui_blood (Utilities|Casting|CastToUI_Blood (UserInterface|GetWidget (Variables|Default|GetHeadWidgetComponent))))
  (return _asui_blood))

(fn SetDecalVisibility
  (params (Visibility :type Boolean))
  (Rendering|SetVisibility (Variables|Default|GetDecalComponent) Visibility false))