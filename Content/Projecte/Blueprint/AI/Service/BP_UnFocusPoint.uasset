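; Behavior tree service for BP_Boss that runs a countdown, apparently for losing focus on an enemy.
; Each tick clears a blackboard bool, then passes the blackboard counter's ratio to MaxCount into the boss's UnFindEnemy and decrements the counter.
; Once the counter drops below zero, it makes the boss's decal visible instead.
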(event EventReceiveTickAI
  (params (OwnerController :type AI%20Controller%20Object%20Reference) (ControlledPawn :type Pawn%20Object%20Reference) (DeltaSeconds :type Float%20%28single-precision%29))
  (bind _keyselector_int (Variables|Default|GetKeySelector_Int))
  (bind _keyselector_bool (Variables|Default|GetKeySelector_Bool))
  (bind _keyselector_int_2 (Variables|Default|GetKeySelector_Int))
  (bind _returnvalue (Class|BTFunctionLibrary|GetBlackboardValueasInt _keyselector_int))
  (bind _asbp_boss (Utilities|Casting|CastToBP_Boss ControlledPawn))
  (Utilities|FlowControl|Sequence
    (:then_0
      (if (Class|BTFunctionLibrary|GetBlackboardValueasBool _keyselector_bool)
        (Class|BTFunctionLibrary|SetBlackboardValueasBool _keyselector_bool false)))
    (:then_1
      (if (< _returnvalue 0)
        (Default|SetDecalVisibility _asbp_boss true)
        (else
          (Default|UnFindEnemy _asbp_boss (/ (Math|Conversions|ToFloat(Integer) _returnvalue) (Math|Conversions|ToFloat(Integer) (Variables|Default|GetMaxCount))))
          (Class|BTFunctionLibrary|SetBlackboardValueasInt _keyselector_int_2 (- (Class|BTFunctionLibrary|GetBlackboardValueasInt _keyselector_int_2) 1)))))))