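; Behavior tree service that runs the boss's timed focus phase, driving its find-enemy call on each tick.
; While an integer blackboard counter is at or below MaxCount, it passes the counter-to-MaxCount ratio to RunFindEnemy on BP_Boss and increments the counter.
; Once the counter exceeds the limit, it sets a blackboard bool and hides the boss's decal, using that bool to do so only once.
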(event EventReceiveTickAI
  (params (OwnerController :type AI%20Controller%20Object%20Reference) (ControlledPawn :type Pawn%20Object%20Reference) (DeltaSeconds :type Float%20%28single-precision%29))
  (bind _keyselector_int (Variables|Default|GetKeySelector_Int))
  (bind _maxcount (Variables|Default|GetMaxCount))
  (bind _keyselector_bool (Variables|Default|GetKeySelector_Bool))
  (bind _keyselector_int_2 (Variables|Default|GetKeySelector_Int))
  (bind _returnvalue (Class|BTFunctionLibrary|GetBlackboardValueasInt _keyselector_int))
  (bind _asbp_boss (Utilities|Casting|CastToBP_Boss ControlledPawn))
  (if (> _returnvalue _maxcount)
    (if (not (Class|BTFunctionLibrary|GetBlackboardValueasBool _keyselector_bool))
      (Class|BTFunctionLibrary|SetBlackboardValueasBool _keyselector_bool true)
      (Default|SetDecalVisibility _asbp_boss false))
    (else
      (Default|RunFindEnemy _asbp_boss (/ (Math|Conversions|ToFloat(Integer) _returnvalue) (Math|Conversions|ToFloat(Integer) _maxcount)))
      (Class|BTFunctionLibrary|SetBlackboardValueasInt _keyselector_int_2 (+ (Class|BTFunctionLibrary|GetBlackboardValueasInt _keyselector_int_2) 1)))))