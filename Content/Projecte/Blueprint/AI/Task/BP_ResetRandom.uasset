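; Behavior tree task that resets the random number on BP_Boss.
; If the boss has AnimPlay set, it waits briefly and finishes as failed without changing the number.
; Otherwise it sets either a random integer from 0 to 5 or the task's own RandomNum, chosen by the Random flag, then finishes successfully after a short delay.
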(event EventReceiveExecuteAI
  (params (OwnerController :type AI%20Controller%20Object%20Reference) (ControlledPawn :type Pawn%20Object%20Reference))
  (bind _asbp_boss (Utilities|Casting|CastToBP_Boss ControlledPawn))
  (if (Variables|/Script/MyRPGGame.EnemyCharacter|GetAnimPlay _asbp_boss)
    (Utilities|FlowControl|Delay 0.2)
    (AI|BehaviorTree|FinishExecute false)
    (else
      (Class|EnemyCharacter|SetRandomNum _asbp_boss (Math|Integer|SelectInt (Math|Random|RandomInteger 6) (Variables|Default|GetRandomNum) (Variables|Default|GetbRandom)))
      (Utilities|FlowControl|Delay 1.0)
      (AI|BehaviorTree|FinishExecute true))))