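; Behavior tree task that counts repeats for the boss and toggles its sit state once the limit is reached.
; While the Count key is below five, it writes that value plus one to RepeatCount and finishes successfully.
; Otherwise it sets the inverse of IsSit on BP_Boss and the Sit key, resets RepeatCount and finishes as failed.
; Reads use key variables, while writes use hard-coded key names.
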(event EventReceiveExecuteAI
  (params (OwnerController :type AI%20Controller%20Object%20Reference) (ControlledPawn :type Pawn%20Object%20Reference))
  (bind _returnvalue (AI|GetBlackboard ControlledPawn))
  (bind _count (Variables|Default|GetCount))
  (bind _repeatcount (Variables|Default|GetRepeatCount))
  (bind _issit (Variables|Default|GetIsSit))
  (bind _returnvalue_2 (Class|BTFunctionLibrary|GetBlackboardValueasBool _issit))
  (bind _returnvalue_3 (Class|BTFunctionLibrary|GetBlackboardValueasInt _count))
  (bind _returnvalue_4 (not _returnvalue_2))
  (if (< _returnvalue_3 5)
    (Class|BlackboardComponent|SetValueasInt _returnvalue _repeatcount (+ _returnvalue_3 1))
    (AI|BehaviorTree|FinishExecute true)
    (else
      (Class|EnemyCharacter|SetSit (.AsBP%20Boss (Utilities|Casting|CastToBP_Boss ControlledPawn)) _returnvalue_4)
      (AI|Components|Blackboard|SetValueasBool _returnvalue (Variables|Default|GetSit) _returnvalue_4)
      (Class|BlackboardComponent|SetValueasInt _returnvalue _repeatcount)
      (AI|BehaviorTree|FinishExecute false))))