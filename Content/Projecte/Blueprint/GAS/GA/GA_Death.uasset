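; GA_Death is the player death gameplay ability in the Gameplay Ability System.
; On activation it opens the HUD death widget, switches input to UI-only with a visible cursor, cancels targeting and adds the death tag.
; It plays the death montage, then on completion ragdolls the mesh and disables capsule collision.
; After a short delay it unpossesses the controller and destroys the owning character.
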(event Ability|EventActivateAbility
  (bind _returnvalue (Ability|GetActorInfo))
  (bind (_owneractor _avataractor _playercontroller _abilitysystemcomponent _skeletalmeshcomponent) (Utilities|Struct|BreakGameplayAbilityActorInfo _returnvalue))
  (bind _asplayer_character (Utilities|Casting|CastToPlayerCharacter _owneractor))
  (Class|PlayerHUD|OpenDeathWidget (.AsPlayer%20HUD (Utilities|Casting|CastToPlayerHUD (HUD|GetHUD _playercontroller))) true)
  (Variables|/Script/Engine.PlayerController|SetbShowMouseCursor _playercontroller true)
  (Input|SetInputModeUIOnly _playercontroller 0 "DoNotLock")
  (Class|TargetComponent|CancelTarget (Variables|/Script/MyRPGGame.PlayerCharacter|GetTargetComponent _asplayer_character))
  (GameplayTags|AddGameplayTag (Variables|/Script/MyRPGGame.BaseCharacter|GetTagContainer _asplayer_character) "(TagName=\"Ability.Player.Death\")" :!class /Script/GameplayTags.BlueprintGameplayTagLibrary)
  (Animation|Montage|PlayMontage _skeletalmeshcomponent "/Game/Projecte/Animation/Character/AnimMontage/AM_Death.AM_Death"
    (:OnCompleted
      (Class|SkeletalMeshComponent|SetAllBodiesSimulatePhysics _skeletalmeshcomponent true)
      (Class|SkeletalMeshComponent|SetAllBodiesPhysicsBlendWeight _skeletalmeshcomponent 1.0 false)
      (Collision|SetCollisionEnabled (Variables|/Script/Engine.Character|GetCapsuleComponent _asplayer_character) "NoCollision")
      (Utilities|FlowControl|Delay 5.0)
      (Pawn|UnPossess _playercontroller)
      (Actor|DestroyActor _owneractor))))

(event Ability|EventOnEndAbility
  (params (bWasCancelled :type Boolean)))