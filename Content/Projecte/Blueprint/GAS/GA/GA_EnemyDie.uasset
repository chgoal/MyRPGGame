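; GA_EnemyDie is a gameplay ability that runs an enemy's death sequence.
; On activation it casts the owner to EnemyCharacter, calls UnPossess on its LastHitBy controller (not the enemy's own controller) and plays the death montage.
; When the montage completes, the mesh switches to full ragdoll physics, capsule collision turns off, and the actor is destroyed after a short delay.
; The ability never explicitly calls EndAbility.
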(event Ability|EventActivateAbility
  (bind _asenemy_character (Utilities|Casting|CastToEnemyCharacter (.OwnerActor (Utilities|Struct|BreakGameplayAbilityActorInfo (Ability|GetActorInfo)))))
  (Pawn|UnPossess (Variables|/Script/Engine.Pawn|GetLastHitBy _asenemy_character))
  (Animation|Montage|PlayMontage 0 "/Game/Projecte/Animation/Enemy/AnimMontage/AM_Death.AM_Death"
    (:OnCompleted
      (Class|SkeletalMeshComponent|SetAllBodiesSimulatePhysics (Variables|/Script/Engine.Character|GetMesh _asenemy_character) true)
      (Class|SkeletalMeshComponent|SetAllBodiesPhysicsBlendWeight (Variables|/Script/Engine.Character|GetMesh _asenemy_character) 1.0 false)
      (Collision|SetCollisionEnabled (Variables|/Script/Engine.Character|GetCapsuleComponent _asenemy_character) "NoCollision")
      (Utilities|FlowControl|Delay 4.0)
      (Actor|DestroyActor _asenemy_character))))

(event Ability|EventOnEndAbility
  (params (bWasCancelled :type Boolean)))