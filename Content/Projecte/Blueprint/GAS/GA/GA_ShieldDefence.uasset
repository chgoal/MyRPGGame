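; Gameplay ability that resolves the player's shield defence against a hit, based on an owner attribute, apparently stamina.
; While that attribute is above zero, it applies the successful-block effect to drain it and plays the shield-hurt montage from a section matching the hit direction.
; Otherwise the guard breaks: it clears RightAttack and the shield tag, then calls MakeDamage on the player with a fixed amount.
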(event Ability|EventActivateAbility
  (bind _returnvalue (Ability|GetActorInfo))
  (bind (_owneractor _avataractor _playercontroller _abilitysystemcomponent _skeletalmeshcomponent) (Utilities|Struct|BreakGameplayAbilityActorInfo _returnvalue))
  (bind _asplayer_character (Utilities|Casting|CastToPlayerCharacter _owneractor))
  (if (> (.ReturnValue (Ability|Attribute|GetFloatAttributefromAbilitySystemComponent _abilitysystemcomponent "(AttributeName=\"Stamina\",Attribute=/Script/MyRPGGame.CharacterAttributeSet:Stamina,AttributeOwner=None)")) 0.0)
    (Ability|ApplyGameplayEffectToOwner "/Game/Projecte/Blueprint/GAS/GE/GE_SucessShield.GE_SucessShield_C") ; 降低部分体力
    (Animation|Montage|PlayMontage _skeletalmeshcomponent "/Game/Projecte/Animation/Character/AnimMontage/AM_ShieldHurt.AM_ShieldHurt" 1.0 0.0 (CallFunction|HitDirectionTransform (Class|BaseCharacter|GetHitDirection _asplayer_character)))
    (else
      (Variables|/Script/MyRPGGame.PlayerCharacter|SetbRightAttack _asplayer_character false)
      (GameplayTags|RemoveGameplayTag (Variables|/Script/MyRPGGame.BaseCharacter|GetTagContainer _asplayer_character) "(TagName=\"Ability.Player.Sword.shield\")" :!class /Script/GameplayTags.BlueprintGameplayTagLibrary)
      (Class|BaseCharacter|MakeDamage _asplayer_character 2e+01))))

(event Ability|EventOnEndAbility
  (params (bWasCancelled :type Boolean)))

(fn HitDirectionTransform
  (params (HitDirection :type EHitDirection%20Enum :default "EHD_Forward"))
  (return (Utilities|Select :Index HitDirection :EHD_Forward "Hurt_FW" :EHD_Right "Hurt_R" :EHD_Left "Hurt_L" :EHD_Backward "Hurt_BW")))