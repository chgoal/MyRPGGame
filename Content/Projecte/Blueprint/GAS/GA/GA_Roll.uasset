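; GA_Roll is a Gameplay Ability that runs the player's roll on BP_Player.
; On activation it adds the roll tag and copies current movement input into MoveX/MoveY when locked on, otherwise zeroing them.
; If an owner attribute exceeds a threshold, it applies GE_Roll and holds the Sprite flag for a short delay.
; The tag is removed only on that branch, and EndAbility is never called.
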(event Ability|EventActivateAbility
  (bind _returnvalue (Ability|GetActorInfo))
  (bind (_owneractor _avataractor _playercontroller _abilitysystemcomponent) (Utilities|Struct|BreakGameplayAbilityActorInfo _returnvalue))
  (bind _asbp_player (Utilities|Casting|CastToBP_Player _owneractor))
  (GameplayTags|AddGameplayTag (Variables|/Script/MyRPGGame.BaseCharacter|GetTagContainer _asbp_player) "(TagName=\"Ability.Player.Roll\")" :!class /Script/GameplayTags.BlueprintGameplayTagLibrary)
  (if (and (== (Variables|/Script/MyRPGGame.BaseCharacter|GetCMoveX _asbp_player) 0.0) (== (Variables|/Script/MyRPGGame.BaseCharacter|GetCMoveY _asbp_player) 0.0))
    (Variables|/Script/MyRPGGame.BaseCharacter|SetMoveX _asbp_player 0.0)
    (Variables|/Script/MyRPGGame.BaseCharacter|SetMoveY _asbp_player 0.0)
    (elif (Class|PlayerCharacter|GetbLockon _asbp_player)
      (Variables|/Script/MyRPGGame.BaseCharacter|SetMoveX _asbp_player (Variables|/Script/MyRPGGame.BaseCharacter|GetCMoveX _asbp_player))
      (Variables|/Script/MyRPGGame.BaseCharacter|SetMoveY _asbp_player (Variables|/Script/MyRPGGame.BaseCharacter|GetCMoveY _asbp_player))
      (else
        (Variables|/Script/MyRPGGame.BaseCharacter|SetMoveX _asbp_player 0.0)
        (Variables|/Script/MyRPGGame.BaseCharacter|SetMoveY _asbp_player 0.0))))
  (if (> (.ReturnValue (Ability|Attribute|GetFloatAttributefromAbilitySystemComponent _abilitysystemcomponent "(AttributeName=\"Stamina\",Attribute=/Script/MyRPGGame.CharacterAttributeSet:Stamina,AttributeOwner=None)")) 3e+01)
    (Variables|/Script/MyRPGGame.PlayerCharacter|SetbSprite _asbp_player true)
    (Ability|ApplyGameplayEffectToOwner "/Game/Projecte/Blueprint/GAS/GE/GE_Roll.GE_Roll_C")
    (Utilities|FlowControl|Delay 0.8)
    (Variables|/Script/MyRPGGame.PlayerCharacter|SetbSprite _asbp_player false)
    (GameplayTags|RemoveGameplayTag (Variables|/Script/MyRPGGame.BaseCharacter|GetTagContainer _asbp_player) "(TagName=\"Ability.Player.Roll\")" :!class /Script/GameplayTags.BlueprintGameplayTagLibrary)))

(event Ability|EventOnEndAbility
  (params (bWasCancelled :type Boolean)))